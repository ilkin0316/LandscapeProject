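; Street lamp actor for the Venice fast building set, with a point light configurable per placed instance.
; The construction script applies exposed variables to the point light's visibility, color, intensity and shadow casting.
; The event graph holds only disabled default events, so the lamp has no runtime logic.
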(event EventBeginPlay)

(event Collision|EventActorBeginOverlap
  (params (OtherActor :type Actor%20Object%20Reference)))

(event EventTick
  (params (DeltaSeconds :type Float%20%28single-precision%29)))

(fn ConstructionScript
  (Rendering|SetVisibility (Variables|Default|GetPointLight) (Variables|Default|Getlight) false)
  (Rendering|Components|Light|SetLightColor (Variables|Default|GetPointLight) (Variables|Default|Getcolor) true)
  (Rendering|Components|Light|SetIntensity (Variables|Default|GetPointLight) (Variables|Default|Getintensity))
  (Rendering|Components|Light|SetCastShadows (Variables|Default|GetPointLight) (Variables|Default|Getcast%20shadows)))