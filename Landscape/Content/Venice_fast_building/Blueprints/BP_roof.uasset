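; Procedural modular roof for the Venice fast-building kit, assembled entirely in the Construction Script from static mesh components.
; Width selects the end and middle meshes, and Length sets how many middle segments repeat between the two ends.
; Dormer entries place single, side-switched or double dormers per segment, with wall or brick material.
; Segments without dormers can receive seeded random chimneys and vents, positioned on roof-mesh sockets.
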(event EventBeginPlay)

(event Collision|EventActorBeginOverlap
  (params (OtherActor :type Actor%20Object%20Reference)))

(event EventTick
  (params (DeltaSeconds :type Float%20%28single-precision%29)))

(fn ConstructionScript
  (bind _width (Variables|Default|Getwidth))
  (bind _dormers (Variables|Default|GetDormers))
  (bind _length (Variables|Default|Getlength))
  (bind _returnvalue (Utilities|Array|Length _dormers))
  (bind _returnvalue_2 (Math|Conversions|ToInteger(Byte) _width))
  (Math|Integer|CompareInt (Class|KismetMathLibrary|BreakRandomStream (Variables|Default|GetSeed))
    (:>
      _)
    (:==
      (Class|KismetMathLibrary|SeedRandomStream (Variables|Default|GetSeed)))
    (:<
      _))
  (bind _returnvalue_3 (AddComponent|AddStaticMeshComponent false))
  (Components|StaticMesh|SetStaticMesh _returnvalue_3 (Utilities|Array|Get(acopy) (Variables|Default|Getroofs_side) _returnvalue_2))
  (for _index (range 1 _length)
    (bind _returnvalue_4 (AddComponent|AddStaticMeshComponent false (Math|Transform|MakeTransform (Math|Vector|MakeVector 0.0 (* _index -3e+02) 0.0))))
    (Components|StaticMesh|SetStaticMesh _returnvalue_4 (Utilities|Array|Get(acopy) (Variables|Default|Getroofs) (Math|Conversions|ToInteger(Byte) (Variables|Default|Getwidth))))
    (Math|Integer|CompareInt _returnvalue
      (:>
        (bind _index_2 (Utilities|FlowControl|ForLoopwithBreak 0 (- _returnvalue 1) :!label _label)
          (:LoopBody
            (Math|Integer|CompareInt (.position (Utilities|Array|Get(acopy) (Variables|Default|GetDormers) _index_2)) _index
              (:==
                (Variables|Default|Setspawned true)
                (switch int (Math|Conversions|ToInteger(Byte) (Variables|Default|Getwidth))
                  (:0
                    (if (.double (Utilities|Array|Get(acopy) (Variables|Default|GetDormers) _index_2))
                      (for _index_3 (range 0 1)
                        (switch int _index_3
                          (:0
                            (bind _returnvalue_5 (AddComponent|AddStaticMeshComponent false (Math|Transform|MakeTransform (Math|Vector|MakeVector 0.0 (* _index -3e+02) 0.0)))))
                          (:1
                            (bind _returnvalue_6 (AddComponent|AddStaticMeshComponent false (Math|Transform|MakeTransform (Math|Vector|MakeVector (* (+ (Math|Conversions|ToInteger(Byte) (Variables|Default|Getwidth)) 3) -3e+02) (* (+ _index 1) -3e+02) 0.0) (Math|Rotator|MakeRotator 0.0 0.0 (- 1.8e+02 0.0001)))))))
                        (if (Variables|Default|GetWall_or_Brck_MAT)
                          (Rendering|Material|SetMaterialbyName _returnvalue_5 "M_wall" (Utilities|Array|Get(acopy) (Variables|Default|GetWall%20MATs) (Math|Conversions|ToInteger(Byte) (Variables|Default|GetWall_MAT))))
                          (else
                            (Rendering|Material|SetMaterialbyName _returnvalue_5 "M_wall" "/Game/Venice_fast_building/Materials/MI_brick_wall_01.MI_brick_wall_01"))))
                      (goto _label Break)
                      (elif (.switchside (Utilities|Array|Get(acopy) (Variables|Default|GetDormers) _index_2))
                        (bind _returnvalue_7 (AddComponent|AddStaticMeshComponent false (Math|Transform|MakeTransform (Math|Vector|MakeVector (* (+ (Math|Conversions|ToInteger(Byte) (Variables|Default|Getwidth)) 3) -3e+02) (* (+ _index 1) -3e+02) 0.0) (Math|Rotator|MakeRotator 0.0 0.0 (- 1.8e+02 0.0001)))))
                        (else
                          (bind _returnvalue_8 (AddComponent|AddStaticMeshComponent false (Math|Transform|MakeTransform (Math|Vector|MakeVector 0.0 (* _index -3e+02) 0.0))))))))
                  (:1
                    (if (.double (Utilities|Array|Get(acopy) (Variables|Default|GetDormers) _index_2))
                      (for _index_4 (range 0 1)
                        (switch int _index_4
                          (:0
                            (bind _returnvalue_9 (AddComponent|AddStaticMeshComponent false (Math|Transform|MakeTransform (Math|Vector|MakeVector 0.0 (* _index -3e+02) 0.0)))))
                          (:1
                            (bind _returnvalue_10 (AddComponent|AddStaticMeshComponent false (Math|Transform|MakeTransform (Math|Vector|MakeVector (* (+ (Math|Conversions|ToInteger(Byte) (Variables|Default|Getwidth)) 3) -3e+02) (* (+ _index 1) -3e+02) 0.0) (Math|Rotator|MakeRotator 0.0 0.0 (- 1.8e+02 0.0001)))))))
                        (if (Variables|Default|GetWall_or_Brck_MAT)
                          (Rendering|Material|SetMaterialbyName _returnvalue_8 "M_wall" (Utilities|Array|Get(acopy) (Variables|Default|GetWall%20MATs) (Math|Conversions|ToInteger(Byte) (Variables|Default|GetWall_MAT))))
                          (else
                            (Rendering|Material|SetMaterialbyName _returnvalue_8 "M_wall" "/Game/Venice_fast_building/Materials/MI_brick_wall_01.MI_brick_wall_01"))))
                      (goto _label Break)
                      (elif (.switchside (Utilities|Array|Get(acopy) (Variables|Default|GetDormers) _index_2))
                        (bind _returnvalue_11 (AddComponent|AddStaticMeshComponent false (Math|Transform|MakeTransform (Math|Vector|MakeVector (* (+ (Math|Conversions|ToInteger(Byte) (Variables|Default|Getwidth)) 3) -3e+02) (* (+ _index 1) -3e+02) 0.0) (Math|Rotator|MakeRotator 0.0 0.0 (- 1.8e+02 0.0001)))))
                        (else
                          (bind _returnvalue_12 (AddComponent|AddStaticMeshComponent false (Math|Transform|MakeTransform (Math|Vector|MakeVector 0.0 (* _index -3e+02) 0.0)))))))))
                (if (Variables|Default|GetWall_or_Brck_MAT)
                  (Rendering|Material|SetMaterialbyName _returnvalue_8 "M_wall" (Utilities|Array|Get(acopy) (Variables|Default|GetWall%20MATs) (Math|Conversions|ToInteger(Byte) (Variables|Default|GetWall_MAT))))
                  (else
                    (Rendering|Material|SetMaterialbyName _returnvalue_8 "M_wall" "/Game/Venice_fast_building/Materials/MI_brick_wall_01.MI_brick_wall_01"))))))
          (:Completed
            (if (Variables|Default|Getspawned)
              (Variables|Default|Setspawned false)
              (else
                (if (Variables|Default|GetRND_chimneys) :!label _label_2
                  (if (Math|Random|RandomBoolfromStream (Variables|Default|GetSeed))
                    (bind _returnvalue_13 (AddComponent|AddStaticMeshComponent false (Math|Transform|MakeTransform (.Location (Math|Transform|BreakTransform (Math|Transform|ComposeTransforms (Transformation|GetSocketTransform _returnvalue_4 (Utilities|Array|Get(acopy) (Transformation|GetAllSocketNames _returnvalue_4) (Math|Random|RandomIntegerinRangefromStream (Variables|Default|GetSeed) 0 1)) "RTS_Component") (Math|Transform|MakeTransform (Math|Vector|MakeVector 0.0 (* _index -3e+02) 0.0))))) (Math|Rotator|MakeRotator (.roll (.Rotation (Math|Transform|BreakTransform (Math|Transform|ComposeTransforms (Transformation|GetSocketTransform _returnvalue_4 (Utilities|Array|Get(acopy) (Transformation|GetAllSocketNames _returnvalue_4) (Math|Random|RandomIntegerinRangefromStream (Variables|Default|GetSeed) 0 1)) "RTS_Component") (Math|Transform|MakeTransform (Math|Vector|MakeVector 0.0 (* _index -3e+02) 0.0)))))) (.pitch (.Rotation (Math|Transform|BreakTransform (Math|Transform|ComposeTransforms (Transformation|GetSocketTransform _returnvalue_4 (Utilities|Array|Get(acopy) (Transformation|GetAllSocketNames _returnvalue_4) (Math|Random|RandomIntegerinRangefromStream (Variables|Default|GetSeed) 0 1)) "RTS_Component") (Math|Transform|MakeTransform (Math|Vector|MakeVector 0.0 (* _index -3e+02) 0.0)))))) (+ (.yaw (.Rotation (Math|Transform|BreakTransform (Math|Transform|ComposeTransforms (Transformation|GetSocketTransform _returnvalue_4 (Utilities|Array|Get(acopy) (Transformation|GetAllSocketNames _returnvalue_4) (Math|Random|RandomIntegerinRangefromStream (Variables|Default|GetSeed) 0 1)) "RTS_Component") (Math|Transform|MakeTransform (Math|Vector|MakeVector 0.0 (* _index -3e+02) 0.0)))))) (Math|Float|SelectFloat 0.0 9e+01 (Math|Random|RandomBoolfromStream (Variables|Default|GetSeed))))) (.Scale (Math|Transform|BreakTransform (Math|Transform|ComposeTransforms (Transformation|GetSocketTransform _returnvalue_4 (Utilities|Array|Get(acopy) (Transformation|GetAllSocketNames _returnvalue_4) (Math|Random|RandomIntegerinRangefromStream (Variables|Default|GetSeed) 0 1)) "RTS_Component") (Math|Transform|MakeTransform (Math|Vector|MakeVector 0.0 (* _index -3e+02) 0.0))))))))
                    (Components|StaticMesh|SetStaticMesh _returnvalue_13 (Utilities|Array|Get(acopy) (Variables|Default|GetChimneys) (Math|Random|RandomIntegerinRangefromStream (Variables|Default|GetSeed) 0 3)))
                    (Rendering|Material|SetMaterialbyName _returnvalue_13 "M_wall" (Utilities|Array|Get(acopy) (Variables|Default|GetWall%20MATs) (Math|Conversions|ToInteger(Byte) (Variables|Default|GetWall_MAT))))))
                (if (Variables|Default|GetRND_vents)
                  (if (Math|Random|RandomBoolfromStream (Variables|Default|GetSeed))
                    (AddComponent|AddStaticMeshComponent false (Math|Transform|ComposeTransforms (Transformation|GetSocketTransform _returnvalue_4 (Utilities|Array|Get(acopy) (Transformation|GetAllSocketNames _returnvalue_4) (Math|Random|RandomIntegerinRangefromStream (Variables|Default|GetSeed) 2 7)) "RTS_Component") (Math|Transform|MakeTransform (Math|Vector|MakeVector 0.0 (* _index -3e+02) 0.0)))))))))))
      (:==
        (goto _label_2))))
  (bind _returnvalue_14 (AddComponent|AddStaticMeshComponent false (Math|Transform|MakeTransform (Math|Vector|MakeVector (* (+ _returnvalue_2 3) -3e+02) (* (+ _length 2) -3e+02) 0.0) (Math|Rotator|MakeRotator 0.0 0.0 (- 1.8e+02 0.0001)))))
  (Components|StaticMesh|SetStaticMesh _returnvalue_14 (Utilities|Array|Get(acopy) (Variables|Default|Getroofs_side) (Math|Conversions|ToInteger(Byte) (Variables|Default|Getwidth)))))