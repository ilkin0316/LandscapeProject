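; BP_bridges is a configurable bridge prop from a fast-building Venice kit, assembled in the Construction Script.
; A BridgesList selection picks the bridge mesh, and an optional wall brick setting applies a color-tinted dynamic material instance to it.
; The first three bridge types also get a matching railing mesh, with a selectable forged railing material.
; The event graph holds no logic.
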(event EventBeginPlay)

(event Collision|EventActorBeginOverlap
  (params (OtherActor :type Actor%20Object%20Reference)))

(event EventTick
  (params (DeltaSeconds :type Float%20%28single-precision%29)))

(fn ConstructionScript
  (bind _bridges_list (Variables|Default|Getbridges%20list))
  (bind _returnvalue (Utilities|Select :Index _bridges_list :NewEnumerator0 0 :NewEnumerator1 1 :NewEnumerator2 2 :NewEnumerator3 3 :NewEnumerator4 4 :NewEnumerator5 5))
  (bind _returnvalue_2 (AddComponent|AddStaticMeshComponent false))
  (Components|StaticMesh|SetStaticMesh _returnvalue_2 (Utilities|Array|Get(acopy) (Variables|Default|Getbridges) _returnvalue))
  (if (Variables|Default|GetWall%20|%20Brick%20MAT)
    (bind _returnvalue_3 (Rendering|Material|CreateDynamicMaterialInstance "/Game/Venice_fast_building/Materials/MI_wall_bridge.MI_wall_bridge" "None" "None" :!class /Script/Engine.KismetMaterialLibrary))
    (Rendering|Material|SetMaterialbyName _returnvalue_2 "M_bridge" _returnvalue_3)
    (Rendering|Material|SetVectorParameterValue _returnvalue_3 "Tint Color" (Math|Conversions|ToLinearColor(Color) (Variables|Default|GetColor)) :!class /Script/Engine.MaterialInstanceDynamic))
  (Math|Integer|CompareInt _returnvalue 3
    (:<
      (bind _returnvalue_4 (AddComponent|AddStaticMeshComponent false))
      (Components|StaticMesh|SetStaticMesh _returnvalue_4 (Utilities|Array|Get(acopy) (Variables|Default|Getbridge_railings) _returnvalue))
      (Rendering|Material|SetMaterial _returnvalue_4 1 (Utilities|Array|Get(acopy) (Variables|Default|Getforged_railing_MATs) (Math|Conversions|ToInteger(Byte) (Variables|Default|Getrailing_MAT)))))))